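; Level game state that holds an intro transition before activating the player's ball pawn.
; BeginPlay waits three seconds, switches the internal state enum, then casts the player pawn to BallLevelBlueprint and calls Activate with false.
; A separate TickTransition function can count the same timer down to that state change, but nothing in this Blueprint calls it.
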(event `self.ReceiveBeginPlay`
  (set `self.TransitionInTimer` 3.0)
  (`KismetSystemLibrary.Delay` (`self.TransitionInTimer`))
  (set `self.InternalState` "NewEnumerator2")
  (bind _asball_level_blueprint (cast `/Game/Blueprints/BallLevelBlueprint` (`GameplayStatics.GetPlayerPawn` 0)))
  (`ActorComponent.Activate` _asball_level_blueprint false))

(fn `TickTransition`
  (params (DeltaTime :type "Float (double-precision)"))
  (if (`|EnumEquality` (`self.InternalState`) "NewEnumerator0")
    (set `self.TransitionInTimer` (- (`self.TransitionInTimer`) DeltaTime))
    (if (<= (`self.TransitionInTimer`) 0.0)
      (set `self.InternalState` "NewEnumerator2"))))

(fn `UserConstructionScript`)