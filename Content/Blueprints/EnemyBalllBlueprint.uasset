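; Enemy ball Blueprint that launches in a random direction via projectile movement and takes damage from bullets.
; Hits spawn particles for red walls, green walls or bullets, and zero health triggers explosion, sound and destruction.
; Tick follows the level GameState, activating the ball during Playing and moving to FinishAnimation on timeout or zero health.
; The finish countdown leads to Results, with delayed reloads of Level1.
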(event `self.ReceiveBeginPlay`
  ;[1 1 1] Starting Velocity and Setting Variables
  (`self.InitialiseVelocity`)
  (bind _asgame_state_level_blueprint (cast `/Game/Blueprints/GameStateLevelBlueprint` (`GameplayStatics.GetGameState`)))
  (set `self.GameStateLevel` _asgame_state_level_blueprint)
  (`ActorComponent.Deactivate`))

(event `self.ReceiveTick`
  (params (DeltaSeconds :type "Float (single-precision)"))
  (bind _finishanimation (`/Game/Blueprints/GameStateLevelBlueprint.FinishAnimation` (`self.GameStateLevel`)))
  (switch `/Game/Blueprints/EGameStateLevel` (`/Game/Blueprints/GameStateLevelBlueprint.InternalState` (`self.GameStateLevel`))
    (:`NewEnumerator2`
      ;[1 1 1] Tick
      (`|ExecutionSequence`
        (:`then_0`
          (`ActorComponent.Activate` false))
        (:`then_1`
          (if (or (<= (`self.SecondsRemaining`) 0.0) (<= (`self.Health`) 0))
            (set `/Game/Blueprints/GameStateLevelBlueprint.InternalState` "NewEnumerator4" (`self.GameStateLevel`))
            (`KismetSystemLibrary.Delay` 3.0)
            (`GameplayStatics.OpenLevel` "Level1")))))
    (:`NewEnumerator4`
      (set `/Game/Blueprints/GameStateLevelBlueprint.FinishAnimation` (- _finishanimation DeltaSeconds) (`self.GameStateLevel`))
      (if (<= _finishanimation 0.0)
        (set `/Game/Blueprints/GameStateLevelBlueprint.InternalState` "NewEnumerator5" (`self.GameStateLevel`))
        (`KismetSystemLibrary.Delay` 3.0)
        (`GameplayStatics.OpenLevel` "Level1")))))

(event `self.ReceiveHit`
  (params (MyComp :type "PrimitiveComponent Object Reference") (Other :type "Actor Object Reference") (OtherComp :type "PrimitiveComponent Object Reference") (bSelfMoved :type Boolean) (HitLocation :type "Object.Vector Structure") (HitNormal :type "Object.Vector Structure") (NormalImpulse :type "Object.Vector Structure") (Hit :type "EngineTypes.HitResult Structure (by ref)"))
  ;[1 1 1] Red/Green wall collisions
  (`self.HandleHitCollisions` Other HitLocation))

(event `InputAction|Pause`
  ;[1 1 1] Pause
  (:`Released`
    (`self.SetPaused` false)))

(fn `DecrementHealth`
  (params (`By amount` :type Integer :default 0))
  (bind _returnvalue (`self.K2_GetActorLocation`))
  (bind _output_get (set `self.Health` (`KismetMathLibrary.Clamp` (- (`self.Health`) `By amount`) 0 100)))
  (if (<= _output_get 0)
    (`GameplayStatics.SpawnEmitterAtLocation` "/Game/StarterContent/Particles/P_Explosion.P_Explosion" _returnvalue)
    (`GameplayStatics.PlaySoundAtLocation` "/Game/SoundEffects/Enemy_Destroyed.Enemy_Destroyed" _returnvalue)
    (`self.K2_DestroyActor`)))

(fn `Get Time Remaining`
  (returns (TimeRemaining :type "Float (double-precision)"))
  (return (`self.SecondsRemaining`)))

(fn `HandleHitCollisions`
  (params (OtherActorRef :type "Actor Object Reference") (Location :type "Object.Vector Structure" :default (0.0 0.0 0.0)))
  (cast `/Game/GameObjects/Parents/RedStaticCollidableBlueprint` OtherActorRef
    (:`then`
      (`GameplayStatics.SpawnEmitterAtLocation` "/Game/Particles/RedParticles.RedParticles" Location))
    (:`CastFailed`
      (cast `/Game/GameObjects/Parents/GreenCollidableBlueprint` OtherActorRef
        (:`then`
          (`GameplayStatics.SpawnEmitterAtLocation` "/Game/Particles/GreenParticles.GreenParticles" Location))
        (:`CastFailed`
          (cast `/Game/Blueprints/Bullet` OtherActorRef)
          (`self.DecrementHealth` 5)
          (`GameplayStatics.SpawnEmitterAtLocation` "/Game/Particles/BulletParticles.BulletParticles" Location))))))

(fn `InitialiseVelocity`
  (set `MovementComponent.Velocity` (* (`KismetMathLibrary.RandomUnitVector`) (`self.Speed`)) (`self.ProjectileMovement1`)))

(fn `SetPaused`
  (params (Pause :type Boolean :default false))
  (bind _output_get (set `self.isPaused` Pause))
  (if _output_get
    (`ActorComponent.Deactivate`)
    (else
      (`ActorComponent.Activate` false))))

(fn `UserConstructionScript`)