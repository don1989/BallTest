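; Bomb actor that explodes on a timer and can be shot down before it goes off.
; Tick counts Timer down, then plays the explosion effect and sounds, spawns a FireBlueprint actor at the bomb's transform and destroys the bomb.
; Hits from Bullet actors reduce clamped Health.
; At zero Health the bomb explodes with the enemy-destroyed sound and is removed without leaving fire.
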(event `self.ReceiveTick`
  (params (DeltaSeconds :type "Float (single-precision)"))
  (`self.Tick` DeltaSeconds))

(event `self.ReceiveHit`
  (params (MyComp :type "PrimitiveComponent Object Reference") (Other :type "Actor Object Reference") (OtherComp :type "PrimitiveComponent Object Reference") (bSelfMoved :type Boolean) (HitLocation :type "Object.Vector Structure") (HitNormal :type "Object.Vector Structure") (NormalImpulse :type "Object.Vector Structure") (Hit :type "EngineTypes.HitResult Structure (by ref)"))
  (`self.HandleHitEvents` Other))

(fn `DecrementHealth`
  (params (ByAmount :type Integer :default 0))
  (bind _returnvalue (`self.K2_GetActorLocation`))
  (bind _output_get (set `self.Health` (`KismetMathLibrary.Clamp` (- (`self.Health`) ByAmount) 0 100)))
  (if (<= _output_get 0)
    (`GameplayStatics.SpawnEmitterAtLocation` "/Game/StarterContent/Particles/P_Explosion.P_Explosion" _returnvalue)
    (`GameplayStatics.PlaySoundAtLocation` "/Game/SoundEffects/Enemy_Destroyed.Enemy_Destroyed" _returnvalue)
    (`self.K2_DestroyActor`)))

(fn `HandleHitEvents`
  (params (ObjectRef :type "Actor Object Reference"))
  (cast `/Game/Blueprints/Bullet` ObjectRef)
  (`self.DecrementHealth` 10))

(fn `Tick`
  (params (DeltaTime :type "Float (double-precision)" :default 0.0))
  (bind _returnvalue (`self.K2_GetActorLocation`))
  (bind _output_get (set `self.Timer` (- (`self.Timer`) DeltaTime)))
  (if (<= _output_get 0.0)
    (`GameplayStatics.SpawnEmitterAtLocation` "/Game/StarterContent/Particles/P_Explosion.P_Explosion" _returnvalue)
    (`GameplayStatics.PlaySoundAtLocation` "/Game/StarterContent/Audio/Explosion02.Explosion02" _returnvalue)
    (`|SpawnActorFromClass` "/Game/Blueprints/FireBlueprint.FireBlueprint_C" (`self.GetTransform`) true)
    (`GameplayStatics.PlaySoundAtLocation` "/Game/SoundEffects/Burning.Burning" _returnvalue)
    (`self.K2_DestroyActor`)))

(fn `UserConstructionScript`)