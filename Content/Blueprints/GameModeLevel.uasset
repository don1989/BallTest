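; Game mode for ball levels that sets up touch controls and first-time tutorials for the selected control scheme.
; On BeginPlay it loads the save game and reads the control mode from the game instance.
; Arcade picks one or two virtual joysticks depending on whether the ball's gun is enabled; Tilt hides sticks and destroys gun powerups.
; Unseen tutorials switch the game state's internal state and are saved as shown.
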(event `self.ReceiveBeginPlay`
  (bind _returnvalue (`GameplayStatics.GetPlayerController` 0))
  (bind _returnvalue_2 (`GameplayStatics.GetGameState`))
  (bind _savegameobject (`self.SaveGameObject`))
  (bind _gameinstance (`self.GameInstance`))
  (bind _returnvalue_3 (`GameplayStatics.LoadGameFromSlot` "SaveGame"))
  (bind _asmy_save_game (cast `/Game/Blueprints/MySaveGame` _returnvalue_3))
  (set `self.SaveGameObject` _asmy_save_game)
  (bind _asmy_game_instance (cast `/Game/Blueprints/MyGameInstance` (`GameplayStatics.GetGameInstance`)))
  (set `self.GameInstance` _asmy_game_instance)
  (bind _output_get (set `self.ControlMode` (`/Game/Blueprints/MyGameInstance.SelectedControl` _asmy_game_instance)))
  (switch `/Game/Blueprints/EControlMode` _output_get
    (:`NewEnumerator0`
      (bind _asball_level_blueprint (cast `/Game/Blueprints/BallLevelBlueprint` (`GameplayStatics.GetPlayerPawn` 0)))
      (if (`/Game/Blueprints/BallLevelBlueprint.isGunEnabled` _asball_level_blueprint)
        (`PlayerController.ActivateTouchInterface` _returnvalue "/Engine/MobileResources/HUD/DefaultVirtualJoysticks.DefaultVirtualJoysticks")
        (else
          (`PlayerController.ActivateTouchInterface` _returnvalue "/Game/UI/LeftVirtualJoystickOnly.LeftVirtualJoystickOnly")))
      (if (not (`/Game/Blueprints/MySaveGame.LeftStickTutorial` (`self.SaveGameObject`)))
        (bind _asgame_state_level_blueprint (cast `/Game/Blueprints/GameStateLevelBlueprint` _returnvalue_2))
        (set `/Game/Blueprints/GameStateLevelBlueprint.InternalState` "NewEnumerator7" _asgame_state_level_blueprint)
        (bind _output_get_2 (set `/Game/Blueprints/MyGameInstance.LeftStickTutorial` true _gameinstance))
        ;[1 1 1] Save
        (set `/Game/Blueprints/MySaveGame.LeftStickTutorial` _output_get_2 _savegameobject)
        (`GameplayStatics.SaveGameToSlot` _savegameobject "SaveGame")))
    (:`NewEnumerator1`
      (`PlayerController.ActivateTouchInterface` (`GameplayStatics.GetPlayerController` 0) "/Game/UI/NoVirtualSticks.NoVirtualSticks")
      (bind _outactors (`GameplayStatics.GetAllActorsOfClass` "/Game/GameObjects/Powerup_GunBlueprint.Powerup_GunBlueprint_C"))
      (for _array_element _outactors
        (`self.K2_DestroyActor` _array_element))
      (if (not (`/Game/Blueprints/MySaveGame.TiltTutorial` (`self.SaveGameObject`)))
        (bind _asgame_state_level_blueprint_2 (cast `/Game/Blueprints/GameStateLevelBlueprint` _returnvalue_2))
        (set `/Game/Blueprints/GameStateLevelBlueprint.InternalState` "NewEnumerator9" _asgame_state_level_blueprint_2)
        (bind _output_get_3 (set `/Game/Blueprints/MyGameInstance.TiltTutorial` true _gameinstance))
        (set `/Game/Blueprints/MySaveGame.TiltTutorial` _output_get_3 _savegameobject)
        (`GameplayStatics.SaveGameToSlot` _savegameobject "SaveGame")))))

(fn `UserConstructionScript`)