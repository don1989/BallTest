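; HUD Blueprint for a ball level that draws the player's stats and game-phase messages as canvas text each frame.
; BeginPlay caches the first ball actor of the GameMode's default pawn class, plus the level GameState.
; DrawHUD polls the ball for spheres remaining, collisions, health and time, showing "Times Up!" at zero.
; GameState's internal state gates the start countdown and a centred score read from the GameMode.
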(event `self.ReceiveBeginPlay`
  ;[1 1 1] Get reference to the ball and gamestate
  (bind _asball_level_blueprint (castclass `/Game/Blueprints/BallLevelBlueprint` (`GameMode.DefaultPawnClass` (`GameplayStatics.GetGameMode`))))
  (bind _outactors (`GameplayStatics.GetAllActorsOfClass` _asball_level_blueprint))
  (set `self.BallRef` (`KismetArrayLibrary.Array_Get` _outactors))
  (bind _asgame_state_level_blueprint (cast `/Game/Blueprints/GameStateLevelBlueprint` (`GameplayStatics.GetGameState`)))
  (set `self.GameStateLevel` _asgame_state_level_blueprint))

(event `self.ReceiveDrawHUD`
  (params (SizeX :type Integer) (SizeY :type Integer))
  (bind _gamestatelevel (`self.GameStateLevel`))
  (bind _ballref (`self.BallRef`))
  (bind _textcolour (`self.TextColour`))
  (bind _returnvalue (`KismetMathLibrary.Conv_IntToDouble` (/ SizeX 2)))
  (`|ExecutionSequence`
    (:`then_0`
      (bind _numspheresremaining (`/Game/Blueprints/BallLevelBlueprint.GetSpheresRemaining` (`self.BallRef`)))
      (`self.DrawText` (`KismetStringLibrary.Concat_StrStr` "Spheres Remaining:" (`KismetStringLibrary.Conv_IntToString` _numspheresremaining)) _textcolour (`KismetMathLibrary.Conv_IntToDouble` (- SizeX 300)) 20.0 null 1.5))
    (:`then_1`
      (bind _numcollisions (`/Game/Blueprints/BallLevelBlueprint.Get Num Collisions` _ballref))
      (`self.DrawText` (`KismetStringLibrary.Concat_StrStr` "Collisions: " (`KismetStringLibrary.Conv_IntToString` _numcollisions)) _textcolour 20.0 20.0 null 1.5))
    (:`then_2`
      (bind _timeremaining (`/Game/Blueprints/BallLevelBlueprint.Get Time Remaining` _ballref))
      (if (<= _timeremaining 0.0)
        (`self.DrawText` "Times Up!" _textcolour _returnvalue 20.0 null 1.5)
        (else
          (`self.DrawText` (`KismetStringLibrary.Concat_StrStr` "Time : " (`KismetStringLibrary.Conv_DoubleToString` _timeremaining)) _textcolour _returnvalue 20.0 null 1.5))))
    (:`then_3`
      (if (`|EnumEquality` (`/Game/Blueprints/GameStateLevelBlueprint.InternalState` (`self.GameStateLevel`)) "NewEnumerator5")
        (bind _asgame_mode_level (cast `/Game/Blueprints/GameModeLevel` (`GameplayStatics.GetGameMode`)))
        (`self.DrawText` (`KismetStringLibrary.Concat_StrStr` "Score: " (`KismetStringLibrary.Conv_IntToString` (`/Game/Blueprints/GameModeLevel.Score` _asgame_mode_level))) _textcolour (`KismetMathLibrary.Conv_IntToDouble` (/ SizeX 2)) (`KismetMathLibrary.Conv_IntToDouble` (/ SizeY 2)) null 1.5)))
    (:`then_4`
      (if (`|EnumEquality` (`/Game/Blueprints/GameStateLevelBlueprint.InternalState` _gamestatelevel) "NewEnumerator0")
        (`self.DrawText` (`KismetStringLibrary.Concat_StrStr` "STARTING IN: " (`KismetStringLibrary.Conv_DoubleToString` (`/Game/Blueprints/GameStateLevelBlueprint.TransitionInTimer` _gamestatelevel))) _textcolour 400.0 400.0 null 1.5)))
    (:`then_5`
      (`self.DrawText` (`KismetStringLibrary.Concat_StrStr` "Health: " (`KismetStringLibrary.Conv_IntToString` (`/Game/Blueprints/BallLevelBlueprint.Health` (`self.BallRef`)))) (struct :`R` 0.11542 :`G` 0.593933 :`B` 0.71 :`A` 1.0) 250.0 20.0 null 1.5))))

(fn `UserConstructionScript`)