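; Spawner actor that periodically drops bombs around the player's ball while the level is playing and the ball's Alarm is at 100 or above.
; BeginPlay caches the level GameState and the first ball actor found.
; Tick accumulates a timer and, at each TimeToSpawn interval, spawns a scaled-up, randomly rotated bomb.
; Its location is randomized within a box around the ball, clamped to X/Y bounds at a set Z.
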(event `self.ReceiveBeginPlay`
  ;[1 1 1] Initialise variables
  (bind _asgame_state_level_blueprint (cast `/Game/Blueprints/GameStateLevelBlueprint` (`GameplayStatics.GetGameState`)))
  (set `self.GameStateLevel` _asgame_state_level_blueprint)
  (bind _outactors (`GameplayStatics.GetAllActorsOfClass` "/Game/Blueprints/BallLevelBlueprint.BallLevelBlueprint_C"))
  (if (> (`KismetArrayLibrary.Array_Length` _outactors) 0)
    (set `self.BallRef` (`KismetArrayLibrary.Array_Get` _outactors))))

(event `self.ReceiveTick`
  (params (DeltaSeconds :type "Float (single-precision)"))
  (switch `/Game/Blueprints/EGameStateLevel` (`/Game/Blueprints/GameStateLevelBlueprint.InternalState` (`self.GameStateLevel`))
    (:`NewEnumerator2`
      (if (>= (`/Game/Blueprints/BallLevelBlueprint.Alarm` (`self.BallRef`)) 100.0)
        (bind _output_get (set `self.CurrentTimer` (+ DeltaSeconds (`self.CurrentTimer`))))
        (if (>= _output_get (`self.TimeToSpawn`))
          (set `self.CurrentTimer` 0.0)
          (`|SpawnActorFromClass` "/Game/Blueprints/BombBlueprint.BombBlueprint_C" (`KismetMathLibrary.MakeTransform` (`KismetMathLibrary.MakeVector` (`KismetMathLibrary.FClamp` (.x (`KismetMathLibrary.RandomPointInBoundingBox` (`self.K2_GetActorLocation` (`self.BallRef`)) (`self.BoxRadius`))) (`self.MinX`) (`self.MaxX`)) (`KismetMathLibrary.FClamp` (.y (`KismetMathLibrary.RandomPointInBoundingBox` (`self.K2_GetActorLocation` (`self.BallRef`)) (`self.BoxRadius`))) (`self.MinY`) (`self.MaxY`)) (`self.Z`)) (`KismetMathLibrary.MakeRot` (`KismetMathLibrary.RandomFloatInRange` 0.0 360.0) (`KismetMathLibrary.RandomFloatInRange` 0.0 360.0) (`KismetMathLibrary.RandomFloatInRange` 0.0 360.0)) (15.0 15.0 15.0)) true))))))

(fn `UserConstructionScript`)